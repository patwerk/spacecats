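; Player controller for the cafe explorer that toggles the pause menu and keeps a list of cats.
; The pause input lazily creates and caches the menu widget, binds its close callback, then shows it with the cursor and Game-and-UI input.
; CloseMenu, triggered by the input or the widget, removes the menu and restores game-only input.
; AddCat appends entries to the Cats array.
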(event Custom|CloseMenu
  (Widget|RemovefromParent (Variables|Default|GetPauseMenu))
  (Variables|Default|SetPauseMenuOpen? false)
  (Variables|Default|SetbShowMouseCursor false)
  (Input|SetInputModeGameOnly self))

(event Input|ActionEvents|InputActionPauseMenu
  (params (Key :type Key%20Structure :default "None"))
  (:Pressed
    (if (Variables|Default|GetPauseMenuOpen?)
      (CallFunction|CloseMenu)
      (else
        (Variables|Default|SetPauseMenuOpen? true)
        (Utilities|IsValid (Variables|Default|GetPauseMenu)
          (:Is%20Valid
            _)
          (:Is%20Not%20Valid
            (bind _returnvalue (UserInterface|CreateWidget "/Game/Blueprints/Widgets/Menu/WBP_PauseMenu.WBP_PauseMenu_C"))
            (bind _output_get (Variables|Default|SetPauseMenu _returnvalue))
            (EventDispatchers|BindEventtoCloseMenu _output_get (delegate Custom|CloseMenu))))
        (UserInterface|Viewport|AddtoViewport (Variables|Default|GetPauseMenu) 0)
        (Input|SetInputModeGameandUI self (Variables|Default|GetPauseMenu) "LockAlways" false)
        (Variables|Default|SetbShowMouseCursor true)))))

(fn ConstructionScript)

(fn AddCat
  (params (NewItem :type BP%20Cat%20Object%20Reference%20%28by%20ref%29))
  (Utilities|Array|Add (Variables|Default|GetCats) NewItem))