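; BP_Cat is a cat actor that blinks, periodically spawns seed pickups and randomizes its body parts on interact.
; Looping timers drive random morph-target blinks and seed spawns.
; TurnOff toggles a timeline-driven glow on body and face materials and point light, and drifts the cat toward a random elevated point with slow spin.
; Sphere overlap briefly sets a follow-player flag, which nothing here reads.
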(event OnComponentEndOverlap(Sphere)
  (params (OverlappedComponent :type Primitive%20Component%20Object%20Reference) (OtherActor :type Actor%20Object%20Reference) (OtherComp :type Primitive%20Component%20Object%20Reference) (OtherBodyIndex :type Integer))
  ;[1 1 1] LookAtPlayerWhen Near
  (Utilities|Casting|CastToP_CafeExplorer OtherActor)
  (Variables|HeadTracking|SetFollowPLayer? false))

(event OnComponentBeginOverlap(Sphere)
  (params (OverlappedComponent :type Primitive%20Component%20Object%20Reference) (OtherActor :type Actor%20Object%20Reference) (OtherComp :type Primitive%20Component%20Object%20Reference) (OtherBodyIndex :type Integer) (bFromSweep :type Boolean) (SweepResult :type Hit%20Result%20Structure%20%28by%20ref%29))
  ;[1 1 1] LookAtPlayerWhen Near
  (Utilities|Casting|CastToP_CafeExplorer OtherActor)
  (Variables|HeadTracking|SetFollowPLayer? true)
  (Utilities|Time|SetTimerbyEvent (delegate Custom|Stop%20LookingAtPlayer) (Math|Random|RandomFloatinRange 2.0 4.0)))

(event Custom|StartBlinking
  ;[1 1 1] Cat Eyes Blinking
  (if (Math|Random|RandomBool)
    (CallFunction|Blink)))

(event Custom|SpawnSeed
  (bind _returnvalue (Transformation|GetActorLocation))
  (if (Math|Random|RandomBool)
    (Game|SpawnActorfromClass "/Game/Blueprints/Interactables/BP_PickupItem.BP_PickupItem_C" (Math|Transform|MakeTransform (Math|Vector|MakeVector (+ (Utilities|RandomSpawnLocationAdd) (.x _returnvalue)) (+ (.y _returnvalue) (Utilities|RandomSpawnLocationAdd)) 0.0) "0, 0, 0" "1,1,1") "Undefined" 0 "NewEnumerator5" "NewEnumerator0" "" false 0)))

(event Custom|Stop%20LookingAtPlayer
  ;[1 1 1] LookAtPlayerWhen Near
  (Variables|HeadTracking|SetFollowPLayer? false))

(event EventTurnOff
  (bind _returnvalue (Transformation|GetActorLocation))
  (Utilities|FlowControl|Sequence
    (:then_0
      ;[1 1 1] Glow
      (if (Variables|Default|GetIsGlowing)
        (CallFunction|StopGlow)
        (else
          (CallFunction|Glow)))
      (Variables|Default|SetIsGlowing (not (Variables|Default|GetIsGlowing))))
    (:then_1
      ;[1 1 1] Hover
      (Variables|Default|SetTargetHoverHeight (Math|Vector|MakeVector (+ (.x _returnvalue) (Math|Random|RandomFloatinRange -1e+02 1e+02)) (+ (.y _returnvalue) (Math|Random|RandomFloatinRange -1e+02 1e+02)) (+ (.z _returnvalue) (Math|Random|RandomFloatinRange 4.5e+02 1.2e+03))))
      (Variables|Default|SetRandomFloatRotation (Math|Random|RandomFloatinRange -1e+01 1e+01))
      (Timeline|Timeline_2 Play
        (:Update
          (Transformation|SetActorLocation (Math|Interpolation|VInterpTo (Transformation|GetActorLocation) (Variables|Default|GetTargetHoverHeight) (Utilities|Time|GetWorldDeltaSeconds) 0.02) false false)
          (Transformation|AddActorLocalRotation (Math|Rotator|MakeRotator (* (Variables|Default|GetRandomFloatRotation) (Utilities|Time|GetWorldDeltaSeconds)) (* (Variables|Default|GetRandomFloatRotation) (Utilities|Time|GetWorldDeltaSeconds)) (* (Variables|Default|GetRandomFloatRotation) (Utilities|Time|GetWorldDeltaSeconds))) false false))))))

(event EventInteract
  (CallFunction|Randomize))

(event EventBeginPlay
  (Utilities|FlowControl|Sequence
    (:then_0
      ;[1 1 1] Cat Eyes Blinking
      (bind _returnvalue (Utilities|Time|SetTimerbyEvent (delegate Custom|StartBlinking) 1.5 true))
      (Variables|Default|SetBlinkingTimer _returnvalue))
    (:then_1
      (Utilities|Time|SetTimerbyEvent (delegate Custom|SpawnSeed) (Variables|Default|GetCatSeedSpawnTime) true))))

(event Custom|Glow
  (bind _newtrack_0 (Timeline|Timeline_0 PlayFromStart)
    (:Update
      (Rendering|Material|SetScalarParameterValue (Variables|Components|GetBodyMat) "Glow" _newtrack_0 :!class /Script/Engine.MaterialInstanceDynamic)
      (Rendering|Components|Light|SetIntensity (Variables|Default|GetPointLight) (* _newtrack_0 (Variables|Default|GetLightIntensityMultiplier)))
      (Rendering|Material|SetScalarParameterValue (Variables|Components|GetFaceMat) "Glow" _newtrack_0 :!class /Script/Engine.MaterialInstanceDynamic))))

(event Custom|StopGlow
  (Utilities|FlowControl|Sequence
    (:then_0
      (bind _newtrack_0 (Timeline|Timeline_0 Stop)
        (:Update
          (Rendering|Material|SetScalarParameterValue (Variables|Components|GetBodyMat) "Glow" _newtrack_0 :!class /Script/Engine.MaterialInstanceDynamic)
          (Rendering|Components|Light|SetIntensity (Variables|Default|GetPointLight) (* _newtrack_0 (Variables|Default|GetLightIntensityMultiplier)))
          (Rendering|Material|SetScalarParameterValue (Variables|Components|GetFaceMat) "Glow" _newtrack_0 :!class /Script/Engine.MaterialInstanceDynamic))))
    (:then_1
      (Timeline|Timeline_1 PlayFromStart
        (:Update
          (bind _returnvalue (Rendering|Material|GetScalarParameterValue (Variables|Components|GetBodyMat) "Glow" :!class /Script/Engine.MaterialInstanceDynamic))
          (Rendering|Material|SetScalarParameterValue (Variables|Components|GetBodyMat) "Glow" (Math|Interpolation|FInterpTo _returnvalue 0.0 (Utilities|Time|GetWorldDeltaSeconds) 1e+01) :!class /Script/Engine.MaterialInstanceDynamic)
          (Rendering|Components|Light|SetIntensity (Variables|Default|GetPointLight) (* (Math|Interpolation|FInterpTo _returnvalue 0.0 (Utilities|Time|GetWorldDeltaSeconds) 1e+01) (Variables|Default|GetLightIntensityMultiplier)))
          (Rendering|Material|SetScalarParameterValue (Variables|Components|GetFaceMat) "Glow" (Math|Interpolation|FInterpTo _returnvalue 0.0 (Utilities|Time|GetWorldDeltaSeconds) 1e+01) :!class /Script/Engine.MaterialInstanceDynamic))))))

(event Custom|Blink
  (bind _morphvalue (Timeline|CloseEyes PlayFromStart)
    (:Update
      (Components|SkeletalMesh|SetMorphTarget (Variables|Default|GetCatHead) "Blinking" _morphvalue false))
    (:Finished
      (bind _morphvalue_2 (Timeline|OpenEyes PlayFromStart)
        (:Update
          (Components|SkeletalMesh|SetMorphTarget (Variables|Default|GetCatHead) "Blinking" _morphvalue_2 false))))))

(fn ConstructionScript
  (Rendering|SetVisibility (Variables|Default|GetSM_Wings) (Variables|Attachments|GetHasWings) false)
  (Rendering|SetVisibility (Variables|Default|GetSM_Antlers) (Variables|Attachments|GetHasAntlers) false))

(fn Randomize
  (bind _meshlistears (Variables|Attachments|GetMeshListEars))
  (bind _meshlistantlers (Variables|Attachments|GetMeshListAntlers))
  (bind _meshlistwings (Variables|Attachments|GetMeshListWings))
  (bind _meshlisttails (Variables|Attachments|GetMeshListTails))
  (Utilities|FlowControl|Sequence
    (:then_0
      (Variables|Attachments|SetHasAntlers (Math|Random|RandomBool))
      (Variables|Attachments|SetHasWings (Math|Random|RandomBool))
      (Components|StaticMesh|SetStaticMesh (Variables|Default|GetSM_Tail) (Utilities|Array|Get(acopy) _meshlisttails (Math|Random|RandomIntegerinRange 0 (- (Utilities|Array|Length _meshlisttails) 1))))
      (Components|StaticMesh|SetStaticMesh (Variables|Default|GetSM_Ears) (Utilities|Array|Get(acopy) _meshlistears (Math|Random|RandomIntegerinRange 0 (- (Utilities|Array|Length _meshlistears) 1))))
      (Components|StaticMesh|SetStaticMesh (Variables|Default|GetSM_Antlers) (Utilities|Array|Get(acopy) _meshlistantlers (Math|Random|RandomIntegerinRange 0 (- (Utilities|Array|Length _meshlistantlers) 1))))
      (Components|StaticMesh|SetStaticMesh (Variables|Default|GetSM_Wings) (Utilities|Array|Get(acopy) _meshlistwings (Math|Random|RandomIntegerinRange 0 (- (Utilities|Array|Length _meshlistwings) 1)))))
    (:then_1
      (Rendering|SetVisibility (Variables|Default|GetSM_Wings) (Variables|Attachments|GetHasWings) false)
      (Rendering|SetVisibility (Variables|Default|GetSM_Antlers) (Variables|Attachments|GetHasAntlers) false))))