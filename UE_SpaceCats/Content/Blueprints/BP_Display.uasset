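; BP_Display is an interactable display that holds up to three plant pots.
; Interact claims the first free of three slots via occupied flags, which this graph never clears, and does nothing once all are taken.
; It spawns a half-scale BP_PlantPot at that slot's transform and attaches it to the display with KeepRelative rules.
; SecondaryAction only prints that no secondary action exists.
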(event EventBeginPlay)

(event Collision|EventActorBeginOverlap
  (params (OtherActor :type Actor%20Object%20Reference)))

(event EventTick
  (params (DeltaSeconds :type Float%20%28single-precision%29)))

(event EventInteract
  (if (Variables|Default|GetLocationOccupied1)
    (if (Variables|Default|GetLocationOccupied2)
      (if (not (Variables|Default|GetLocationOccupied3))
        (Variables|Default|SetItemDisplayLocation (Variables|Default|GetItemDisplayLocation3))
        (Variables|Default|SetLocationOccupied3 true)
        (bind _returnvalue (Game|SpawnActorfromClass "/Game/Blueprints/BP_PlantPot.BP_PlantPot_C" (Math|Transform|MakeTransform (.location (Variables|Default|GetItemDisplayLocation)) (.rotation (Variables|Default|GetItemDisplayLocation)) "0.500000,0.500000,0.500000") "Undefined" 0 "NewEnumerator0" 0 :!label _label))
        (Transformation|AttachActorToActor _returnvalue self "None" "KeepRelative" "KeepRelative" "KeepRelative" true))
      (else
        (Variables|Default|SetItemDisplayLocation (Variables|Default|GetItemDisplayLocation2))
        (Variables|Default|SetLocationOccupied2 true)
        (goto _label)))
    (else
      (Variables|Default|SetItemDisplayLocation (Variables|Default|GetItemDisplayLocation1))
      (Variables|Default|SetLocationOccupied1 true)
      (goto _label))))

(event EventSecondaryAction
  (Development|PrintString "Display no secondary action"))

(fn ConstructionScript)