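; BP_PickupItem is an interactable pickup for a watering can, basket, catnip or seed pack.
; The construction script sets the mesh from ItemType and randomly picks one of three seed types for seeds.
; PickupItem hides the mesh and name text and returns the ItemType instead of destroying the actor.
; ReturnToStart makes the mesh visible and re-enables ShowName, while Interact is an empty event here.
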(event Custom|ReturnToStart
  (Rendering|SetVisibility (Variables|Character|GetMesh) true false)
  (Variables|Default|SetShowName true))

(event EventBeginPlay
  (|CallParentFunction) ; This node is disabled and will not be called.\nDrag off pins to build functionality.
)

(event Collision|EventActorBeginOverlap
  (params (OtherActor :type Actor%20Object%20Reference)))

(event EventTick
  (params (DeltaSeconds :type Float%20%28single-precision%29)))

(event EventInteract)

(fn ConstructionScript
  (|CallParentFunction)
  (switch Utilities|FlowControl|Switch|SwitchonE_ItemInHand (Variables|Default|GetItemType)
    (:NewEnumerator0
      (Components|StaticMesh|SetStaticMesh (Variables|Character|GetMesh) "/Game/meshes/static/gameplay_items/watering_can.watering_can"))
    (:NewEnumerator2
      (Components|StaticMesh|SetStaticMesh (Variables|Character|GetMesh) "/Game/meshes/static/gameplay_items/basket.basket"))
    (:NewEnumerator3
      (Components|StaticMesh|SetStaticMesh (Variables|Character|GetMesh) "/Game/meshes/static/gameplay_items/catnip.catnip"))
    (:NewEnumerator5
      (Components|StaticMesh|SetStaticMesh (Variables|Character|GetMesh) "/Game/meshes/static/gameplay_items/seed_pack.seed_pack")
      (switch int (Math|Random|RandomIntegerinRange 0 2)
        (:0
          (Variables|Default|SetSeedType "NewEnumerator0"))
        (:1
          (Variables|Default|SetSeedType "NewEnumerator10"))
        (:2
          (Variables|Default|SetSeedType "NewEnumerator12"))))
    (:NewEnumerator4
      (Components|StaticMesh|SetStaticMesh (Variables|Character|GetMesh) 0))))

(fn PickupItem
  (Rendering|SetVisibility (Variables|Character|GetMesh) false false)
  (CallFunction|HideWorldTextWidget)
  (Variables|Default|SetShowName false)
  (return (Variables|Default|GetItemType)))