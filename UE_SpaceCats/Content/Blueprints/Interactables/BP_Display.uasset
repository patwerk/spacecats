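; BP_Display is an interactable cafe display that shows copies of the items the player deposits.
; On Interact, it adds a static mesh component at the next PastryLocations transform for each valid hand ingredient and cat item, then destroys those items.
; An empty-handed interaction destroys the last displayed mesh without returning an item.
; Meshes and Index act as a stack, with no capacity check when adding.
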(event EventInteract
  (bind _meshes (Variables|Default|GetMeshes))
  (bind _index (Variables|Default|Getindex))
  (bind _asp_cafe_explorer (Utilities|Casting|CastToP_CafeExplorer (Game|GetPlayerCharacter 0)))
  (if (Math|Boolean|ORBoolean (Utilities|IsValid (Variables|/Game/Blueprints/Player/P_CafeExplorer.P_CafeExplorer_C|GetBPCatitem _asp_cafe_explorer)) (Utilities|IsValid (Variables|/Game/Blueprints/Player/P_CafeExplorer.P_CafeExplorer_C|GetIngredientHand1 _asp_cafe_explorer)) (Utilities|IsValid (Variables|/Game/Blueprints/Player/P_CafeExplorer.P_CafeExplorer_C|GetIngredientHand2 _asp_cafe_explorer)))
    (Utilities|FlowControl|Sequence
      (:then_0
        (Utilities|IsValid (Variables|/Game/Blueprints/Player/P_CafeExplorer.P_CafeExplorer_C|GetIngredientHand1 _asp_cafe_explorer)
          (:Is%20Valid
            (bind _returnvalue (AddComponent|AddStaticMeshComponent false (Utilities|Array|Get(acopy) (Variables|Default|GetPastryLocations) (Variables|Default|Getindex))))
            (Components|StaticMesh|SetStaticMesh _returnvalue (Variables|/Script/Engine.StaticMeshComponent|GetStaticMesh (Variables|/Game/Blueprints/Interactables/BP_Interactable.BP_Interactable_C|GetMesh (Variables|/Game/Blueprints/Player/P_CafeExplorer.P_CafeExplorer_C|GetIngredientHand1 _asp_cafe_explorer))))
            (Utilities|Array|Add (Variables|Default|GetMeshes) _returnvalue)
            (Math|Integer|IncrementInt (Variables|Default|Getindex)))))
      (:then_1
        (Utilities|IsValid (Variables|/Game/Blueprints/Player/P_CafeExplorer.P_CafeExplorer_C|GetIngredientHand2 _asp_cafe_explorer)
          (:Is%20Valid
            (bind _returnvalue_2 (AddComponent|AddStaticMeshComponent false (Utilities|Array|Get(acopy) (Variables|Default|GetPastryLocations) (Variables|Default|Getindex))))
            (Components|StaticMesh|SetStaticMesh _returnvalue_2 (Variables|/Script/Engine.StaticMeshComponent|GetStaticMesh (Variables|/Game/Blueprints/Interactables/BP_Interactable.BP_Interactable_C|GetMesh (Variables|/Game/Blueprints/Player/P_CafeExplorer.P_CafeExplorer_C|GetIngredientHand2 _asp_cafe_explorer))))
            (Utilities|Array|Add (Variables|Default|GetMeshes) _returnvalue_2)
            (Math|Integer|IncrementInt (Variables|Default|Getindex)))))
      (:then_2
        (Utilities|IsValid (Variables|/Game/Blueprints/Player/P_CafeExplorer.P_CafeExplorer_C|GetBPCatitem _asp_cafe_explorer)
          (:Is%20Valid
            (bind _returnvalue_3 (AddComponent|AddStaticMeshComponent false (Utilities|Array|Get(acopy) (Variables|Default|GetPastryLocations) (Variables|Default|Getindex))))
            (Components|StaticMesh|SetStaticMesh _returnvalue_3 (Variables|/Script/Engine.StaticMeshComponent|GetStaticMesh (Variables|/Game/Blueprints/Interactables/BP_Interactable.BP_Interactable_C|GetMesh (Variables|/Game/Blueprints/Player/P_CafeExplorer.P_CafeExplorer_C|GetBPCatitem _asp_cafe_explorer))))
            (Utilities|Array|Add (Variables|Default|GetMeshes) _returnvalue_3)
            (Math|Integer|IncrementInt (Variables|Default|Getindex)))))
      (:then_3
        (Default|DestroyHandItems _asp_cafe_explorer)
        (Default|DestroyCatItem _asp_cafe_explorer)))
    (elif (> (Variables|Default|Getindex) 0)
      (Math|Integer|DecrementInt _index
        (:%20%20
          (Components|DestroyComponent (Utilities|Array|Get(acopy) _meshes _index))
          (Utilities|Array|RemoveIndex _meshes _index))))))

(fn ConstructionScript
  (|CallParentFunction))