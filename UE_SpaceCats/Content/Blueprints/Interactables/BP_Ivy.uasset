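; BP_Ivy is an interactable that gives the cafe explorer player an ingredient.
; On Interact, it casts the player character to P_CafeExplorer and continues only if IngredientHand1 holds no valid ingredient.
; It then spawns a BP_Ingredient of a fixed type, with no display name, below the world origin and stores it in that hand slot.
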(event EventBeginPlay
  (|CallParentFunction) ; This node is disabled and will not be called.\nDrag off pins to build functionality.
)

(event Collision|EventActorBeginOverlap
  (params (OtherActor :type Actor%20Object%20Reference)))

(event EventTick
  (params (DeltaSeconds :type Float%20%28single-precision%29)))

(event EventInteract
  (bind _asp_cafe_explorer (Utilities|Casting|CastToP_CafeExplorer (Game|GetPlayerCharacter 0)))
  (Utilities|IsValid (Variables|/Game/Blueprints/Player/P_CafeExplorer.P_CafeExplorer_C|GetIngredientHand1 _asp_cafe_explorer)
    (:Is%20Not%20Valid
      (bind _returnvalue (Game|SpawnActorfromClass "/Game/Blueprints/Interactables/BP_Ingredient.BP_Ingredient_C" (Math|Transform|MakeTransform "0, 0,-1000.000000") "Undefined" 0 "NewEnumerator23" true "" false 0))
      (Variables|/Game/Blueprints/Player/P_CafeExplorer.P_CafeExplorer_C|SetIngredientHand1 _asp_cafe_explorer _returnvalue))))

(fn ConstructionScript
  (|CallParentFunction))