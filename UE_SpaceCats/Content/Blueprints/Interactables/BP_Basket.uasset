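; BP_Basket is an interactable basket that displays a set of ingredients as spawned BP_Ingredient actors.
; SetIngredients destroys the previous actors, then spawns one per Ingredients entry at numbered skeletal mesh sockets (s_ing_N) and tracks them in ACtorsInBasket.
; HideIngredients and ShowIngredients toggle each spawned mesh's visibility and collision together.
; DestroyHidden destroys invisible ingredients, removing them from the array while iterating it.
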(event Custom|SetIngredients
  (bind _actorsinbasket (Variables|Default|GetACtorsInBasket))
  (for _array_element _actorsinbasket
    (Utilities|IsValid _array_element
      (:Is%20Valid
        (Actor|DestroyActor _array_element))))
  (Utilities|Array|Clear _actorsinbasket)
  (for (_array_element_2 _array_index) (Variables|Default|GetIngredients)
    (bind _returnvalue (Game|SpawnActorfromClass "/Game/Blueprints/Interactables/BP_Ingredient.BP_Ingredient_C" (Math|Transform|MakeTransform (Transformation|GetSocketLocation (Variables|Default|GetSkeletalMesh) (Utilities|String|StringToName (Utilities|String|ToString(Text) (Utilities|Text|FormatText "s_ing_{x}" (+ _array_index 1))))) "0, 0, 0" (Variables|Default|GetIngredientInBasketScale)) "Undefined" 0 _array_element_2 true "" false 0))
    (Utilities|Array|Add (Variables|Default|GetACtorsInBasket) _returnvalue)))

(event Custom|ShowIngredients
  (for _array_element (Variables|Default|GetACtorsInBasket)
    (Utilities|IsValid _array_element
      (:Is%20Valid
        (Rendering|SetVisibility (Variables|/Game/Blueprints/Interactables/BP_Interactable.BP_Interactable_C|GetMesh _array_element) true false)
        (Collision|SetCollisionEnabled (Variables|/Game/Blueprints/Interactables/BP_Interactable.BP_Interactable_C|GetMesh _array_element) "QueryAndPhysics")))))

(event Custom|DestroyHidden
  (for (_array_element _array_index) (Variables|Default|GetACtorsInBasket)
    (if (not (Rendering|IsVisible (Variables|/Game/Blueprints/Interactables/BP_Interactable.BP_Interactable_C|GetMesh _array_element)))
      (Actor|DestroyActor _array_element)
      (Utilities|Array|RemoveIndex (Variables|Default|GetACtorsInBasket) _array_index))))

(event Custom|HideIngredients
  (for _array_element (Variables|Default|GetACtorsInBasket)
    (Utilities|IsValid _array_element
      (:Is%20Valid
        (Rendering|SetVisibility (Variables|/Game/Blueprints/Interactables/BP_Interactable.BP_Interactable_C|GetMesh _array_element) false false)
        (Collision|SetCollisionEnabled (Variables|/Game/Blueprints/Interactables/BP_Interactable.BP_Interactable_C|GetMesh _array_element) "NoCollision")))))

(fn ConstructionScript)