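; Interactable café blender that combines the two ingredients in the player's hands into a new item.
; Interact consumes both items and runs a mixing timeline, then Validate matches the pair against DT_Recipes in either order.
; The result spawns as an attached BP_Catitem, with a failure sound for unmatched pairs, and blocks further use via HasItemWaiting.
; A specific first ingredient plus a base ingredient from DT_Ingredients instead triggers CallCreatedNewCat.
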(event EventInteract
  (bind _returnvalue (Game|GetPlayerCharacter 0))
  (bind _spawnlocation (Variables|Default|GetSpawnLocation))
  (bind _asp_cafe_explorer (Utilities|Casting|CastToP_CafeExplorer _returnvalue))
  (if (Math|Boolean|ANDBoolean (not (Variables|Default|GetHasItemWaiting)) (Utilities|IsValid (Variables|/Game/Blueprints/Player/P_CafeExplorer.P_CafeExplorer_C|GetIngredientHand1 _asp_cafe_explorer)) (Utilities|IsValid (Variables|/Game/Blueprints/Player/P_CafeExplorer.P_CafeExplorer_C|GetIngredientHand2 _asp_cafe_explorer)))
    (Variables|Default|SetIngredient1 (Variables|/Game/Blueprints/Interactables/BP_Ingredient.BP_Ingredient_C|GetIngredientType (Variables|/Game/Blueprints/Player/P_CafeExplorer.P_CafeExplorer_C|GetIngredientHand1 _asp_cafe_explorer)))
    (Variables|Default|SetIngredient2 (Variables|/Game/Blueprints/Interactables/BP_Ingredient.BP_Ingredient_C|GetIngredientType (Variables|/Game/Blueprints/Player/P_CafeExplorer.P_CafeExplorer_C|GetIngredientHand2 _asp_cafe_explorer)))
    (Audio|PlaySoundatLocation "/Game/Blueprints/Audio/SFX/C_mixing.C_mixing" (Transformation|GetActorLocation) "0, 0, 0" 1.0 1.0 0.0 0 0 0)
    (Variables|Default|SetMaking true)
    (Default|DestroyHandItems _asp_cafe_explorer)
    (Timeline|Timeline_0_0 PlayFromStart
      (:Finished
        (Variables|Default|SetMaking false)
        (Utilities|FlowControl|Delay 1.0)
        (bind _returnvalue_2 (Utilities|GetDataTableRow "/Game/Blueprints/Data/DT_Ingredients.DT_Ingredients" (Utilities|String|StringToName (Utilities|String|EnumtoString (Variables|Default|GetIngredient2))))
          (:then
            (if (and (Utilities|Enum|Equal(Enum) (Variables|Default|GetIngredient1) "NewEnumerator23") (.IsBaseIngredient (Utilities|Struct|BreakS_Ingredient _returnvalue_2)))
              (Audio|PlaySoundatLocation "/Game/Blueprints/Audio/SFX/sfx_metamorph_Cue.sfx_metamorph_Cue" (Transformation|GetActorLocation) "0, 0, 0" 1.0 1.5 0.0 "/Game/Blueprints/Audio/Attenuation/Meowing.Meowing" 0 0)
              (Default|CallCreatedNewCat)
              (else
                (bind _newparam (CallFunction|Validate :!label _label))
                (if (Utilities|Enum|Equal(Enum) _newparam "NewEnumerator0")
                  (Audio|PlaySoundatLocation "/Game/Blueprints/Audio/SFX/C_bad_rec.C_bad_rec" (Transformation|GetActorLocation) "0, 0, 0" 1.0 1.0 0.0 0 0 0)
                  (else
                    (Audio|PlaySoundatLocation "/Game/Blueprints/Audio/SFX/C_Result.C_Result" (Transformation|GetActorLocation) "0, 0, 0" 1.0 1.0 0.0 0 0 0)))
                (bind _returnvalue_3 (Game|SpawnActorfromClass "/Game/Blueprints/Interactables/BP_Catitem.BP_Catitem_C" (Math|Transform|MakeTransform (.location _spawnlocation) (.rotation _spawnlocation) "1,1,1") "Undefined" 0 _newparam "" false 0))
                (Transformation|AttachActorToActor _returnvalue_3 self "None" "KeepRelative" "KeepRelative" "KeepRelative" true)
                (Variables|Default|SetHasItemWaiting true))))
          (:RowNotFound
            (goto _label)))))))

(fn ConstructionScript
  (|CallParentFunction))

(fn Validate
  (bind _outrownames (DataTable|GetDataTableRowNames "/Game/Blueprints/Data/DT_Recipes.DT_Recipes"))
  (bind _array_element (Utilities|Array|ForEachLoopwithBreak _outrownames :!label _label)
    (:LoopBody
      (bind _returnvalue (Utilities|GetDataTableRow "/Game/Blueprints/Data/DT_Recipes.DT_Recipes" _array_element)
        (:then
          (if (Utilities|Enum|Equal(Enum) (Variables|Default|GetIngredient1) (.Ingredient_1 (Utilities|Struct|BreakS_Recipe _returnvalue)))
            (if (Utilities|Enum|Equal(Enum) (.Ingredient_2 (Utilities|Struct|BreakS_Recipe _returnvalue)) (Variables|Default|GetIngredient2))
              (LocalVariables|SetResultItem (.Name (Utilities|Struct|BreakS_Recipe _returnvalue)) :!label _label_2)
              (goto _label Break)
              (else
                _))
            (elif (Utilities|Enum|Equal(Enum) (.Ingredient_1 (Utilities|Struct|BreakS_Recipe _returnvalue)) (Variables|Default|GetIngredient2))
              (if (Utilities|Enum|Equal(Enum) (.Ingredient_2 (Utilities|Struct|BreakS_Recipe _returnvalue)) (Variables|Default|GetIngredient1))
                (goto _label_2)
                (else
                  _))))
          (LocalVariables|SetResultItem "NewEnumerator0"))))
    (:Completed
      (return (LocalVariables|GetResultItem)))))