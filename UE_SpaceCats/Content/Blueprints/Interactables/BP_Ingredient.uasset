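; BP_Ingredient is an interactable ingredient that the P_CafeExplorer player character can receive.
; Its construction script looks up the IngredientType row in DT_Ingredients and sets the mesh to the ingredient or world variant based on IsIngredient.
; Primary interact passes the type to the player's ReceiveItem when CatItemInHand matches one specific enum value.
; Secondary interact only prints a debug message after the parent call.
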(event EventBeginPlay)

(event Collision|EventActorBeginOverlap
  (params (OtherActor :type Actor%20Object%20Reference)))

(event EventTick
  (params (DeltaSeconds :type Float%20%28single-precision%29)))

(fn ConstructionScript
  (|CallParentFunction)
  (bind _returnvalue (Utilities|GetDataTableRow "/Game/Blueprints/Data/DT_Ingredients.DT_Ingredients" (Utilities|String|StringToName (Utilities|String|EnumtoString (Variables|Default|GetIngredientType))))
    (:then
      (if (Variables|Default|GetIsIngredient)
        (Components|StaticMesh|SetStaticMesh (Variables|Character|GetMesh) (.IngredientMesh (Utilities|Struct|BreakS_Ingredient _returnvalue)))
        (else
          (Components|StaticMesh|SetStaticMesh (Variables|Character|GetMesh) (.WorldMesh (Utilities|Struct|BreakS_Ingredient _returnvalue))))))))

(fn InteractPrimary
  (|CallParentFunction)
  (bind _asp_cafe_explorer (Utilities|Casting|CastToP_CafeExplorer (Game|GetPlayerCharacter 0)))
  (if (Utilities|Enum|Equal(Enum) (Variables|/Game/Blueprints/Player/P_CafeExplorer.P_CafeExplorer_C|GetCatItemInHand _asp_cafe_explorer) "NewEnumerator2")
    (Default|ReceiveItem _asp_cafe_explorer (Variables|Default|GetIngredientType))))

(fn InteractSecondary
  (|CallParentFunction)
  (Development|PrintString "child secondary message"))