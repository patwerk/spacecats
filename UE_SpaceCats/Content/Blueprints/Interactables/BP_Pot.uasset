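; BP_Pot is an interactable plant pot where the player plants a held seed and waters it to grow an ingredient.
; Planting shows a scaling sprout and starts timers that advance growth stages or kill the plant, resetting the pot.
; Watering restarts the death timer, and enough waterings advance a stage early.
; The final stage spawns an attached BP_Ingredient; the construction script selects the pot mesh.
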(event Custom|PlantDie
  (bind _sproutmesh (Variables|Default|GetSproutMesh))
  (bind _bpplant (Variables|Default|GetBpPlant))
  ;[1 1 1] Cycle of Life and Death
  (if (Utilities|Enum|NotEqual(Enum) (Variables|Default|GetGrowStage) "NewEnumerator4")
    (Variables|Default|SetGrowStage "NewEnumerator4")
    (Rendering|SetVisibility _sproutmesh false false)
    (Transformation|SetRelativeScale3D _sproutmesh "0, 0, 0")
    (Components|StaticMesh|SetStaticMesh _sproutmesh "/Game/meshes/static/plants/sprout_1.sprout_1")
    (Utilities|IsValid _bpplant
      (:Is%20Valid
        (Actor|DestroyActor _bpplant)))))

(event Custom|GrowPlant
  ;[1 1 1] GrowFinalPLant
  (bind _returnvalue (Game|SpawnActorfromClass "/Game/Blueprints/Interactables/BP_Ingredient.BP_Ingredient_C" (Math|Transform|MakeTransform "0, 0, 0" "0, 0, 0" "1,1,1") "Undefined" 0 (Variables|Default|GetPlant) false "BP_Interactable" false 0))
  (Transformation|AttachActorToActor _returnvalue self "None" "KeepRelative" "KeepRelative" "KeepRelative" true)
  (Transformation|SetActorRelativeLocation _returnvalue (Variables|Default|GetPlantSpawn) false true)
  (Variables|Default|SetBpPlant _returnvalue)
  (Audio|PlaySoundatLocation "/Game/Environment/Audio/SFX/RAW/C_Poof.C_Poof" (Transformation|GetActorLocation) "0, 0, 0" 1.0 1.0 0.0 "/Game/Blueprints/Audio/Attenuation/Meowing.Meowing" 0 0)
  (Rendering|SetVisibility (Variables|Default|GetSproutMesh) false false))

(event Custom|GrowNextStage
  ;[1 1 1] Cycle of Life and Death
  (switch Utilities|FlowControl|Switch|SwitchonE_IngredientStage (Variables|Default|GetGrowStage)
    (:NewEnumerator1
      (Variables|Default|SetGrowStage "NewEnumerator2")
      (Components|StaticMesh|SetStaticMesh (Variables|Default|GetSproutMesh) "/Game/meshes/static/plants/sprout_2.sprout_2"))
    (:NewEnumerator2
      (Variables|Default|SetGrowStage "NewEnumerator3")
      (CallFunction|GrowPlant))))

(event Custom|GrowFirstSprout
  ;[1 1 1] Grow First Sprout
  (Rendering|SetVisibility (Variables|Default|GetSproutMesh) true false)
  (Timeline|Timeline_2 PlayFromStart
    (:Update
      (Transformation|SetRelativeScale3D (Variables|Default|GetSproutMesh) (Math|Interpolation|VInterpTo (Variables|/Script/Engine.SceneComponent|GetRelativeScale3D (Variables|Default|GetSproutMesh)) "1.000000,1.000000,1.000000" (Utilities|Time|GetWorldDeltaSeconds) 2.0)))))

(event Custom|StartLifeTimer
  ;[1 1 1] Cycle of Life and Death
  (bind _returnvalue (Utilities|Time|SetTimerbyEvent (delegate Custom|PlantDie) (Variables|Default|GetDieTime) true))
  (Variables|Default|SetDestroyTimer _returnvalue)
  (Utilities|Time|SetTimerbyEvent (delegate Custom|GrowNextStage) (Variables|Default|GetGrowTime) true))

(event EventBeginPlay
  (|CallParentFunction))

(event EventInteract
  (bind _asp_cafe_explorer (Utilities|Casting|CastToP_CafeExplorer (Game|GetPlayerCharacter 0)))
  (Utilities|IsValid (Variables|/Game/Blueprints/Player/P_CafeExplorer.P_CafeExplorer_C|GetItemInHand _asp_cafe_explorer)
    (:Is%20Valid
      (if (Utilities|Enum|Equal(Enum) (Variables|/Game/Blueprints/Interactables/BP_PickupItem.BP_PickupItem_C|GetItemType (Variables|/Game/Blueprints/Player/P_CafeExplorer.P_CafeExplorer_C|GetItemInHand _asp_cafe_explorer)) "NewEnumerator5")
        (Variables|Default|SetPlant (Variables|/Game/Blueprints/Interactables/BP_PickupItem.BP_PickupItem_C|GetSeedType (Variables|/Game/Blueprints/Player/P_CafeExplorer.P_CafeExplorer_C|GetItemInHand _asp_cafe_explorer)))
        ;[1 1 1] SeedInteraction
        (CallFunction|GrowFirstSprout)
        (Variables|/Game/Blueprints/Player/P_CafeExplorer.P_CafeExplorer_C|SetCatItemInHand _asp_cafe_explorer "NewEnumerator4")
        (Actor|DestroyActor (Variables|/Game/Blueprints/Player/P_CafeExplorer.P_CafeExplorer_C|GetItemInHand _asp_cafe_explorer))
        (Variables|Default|SetGrowStage "NewEnumerator1")
        (CallFunction|StartLifeTimer)
        (else
          ;[1 1 1] Watering the plant
          (if (and (Utilities|Enum|Equal(Enum) (Variables|/Game/Blueprints/Interactables/BP_PickupItem.BP_PickupItem_C|GetItemType (Variables|/Game/Blueprints/Player/P_CafeExplorer.P_CafeExplorer_C|GetItemInHand _asp_cafe_explorer)) "NewEnumerator0") (Utilities|Enum|NotEqual(Enum) (Variables|Default|GetGrowStage) "NewEnumerator4"))
            (Utilities|Time|ClearandInvalidateTimerbyHandle (Variables|Default|GetDestroyTimer))
            (bind _returnvalue (Utilities|Time|SetTimerbyEvent (delegate Custom|PlantDie) (Variables|Default|GetDieTime)))
            (Variables|Default|SetDestroyTimer _returnvalue)
            (Math|Integer|IncrementInt (Variables|Default|GetWateredCounter)
              (:%20%20
                (if (>= (Variables|Default|GetWateredCounter) (Variables|Default|GetCheatWateringCount))
                  (Variables|Default|SetWateredCounter 0)
                  (CallFunction|GrowNextStage))))))))))

(fn ConstructionScript
  (|CallParentFunction)
  (Utilities|FlowControl|Sequence
    (:then_0
      (switch Utilities|FlowControl|Switch|SwitchonE_PotStyle (Variables|Default|GetPot)
        (:NewEnumerator0
          (Components|StaticMesh|SetStaticMesh (Variables|Character|GetMesh) "/Game/meshes/static/plant_pots/pot_1.pot_1"))
        (:NewEnumerator1
          (Components|StaticMesh|SetStaticMesh (Variables|Character|GetMesh) "/Game/meshes/static/plant_pots/pot_2.pot_2"))
        (:NewEnumerator2
          (Components|StaticMesh|SetStaticMesh (Variables|Character|GetMesh) "/Game/meshes/static/plant_pots/pot_3.pot_3"))))))