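; Parent interactable Blueprint for objects the cafe explorer pawn can highlight and use.
; Primary and secondary interact events call functions that only print placeholder messages, and highlighting toggles custom depth on the mesh.
; On BeginPlay it passes its name to a WBP_InteractableName widget.
; When ShowName is set, box overlaps with P_CafeExplorer drive timelines that fade the name in and out, and HideWorldTextWidget also fades it out.
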(event OnComponentBeginOverlap(Box)
  (params (OverlappedComponent :type Primitive%20Component%20Object%20Reference) (OtherActor :type Actor%20Object%20Reference) (OtherComp :type Primitive%20Component%20Object%20Reference) (OtherBodyIndex :type Integer) (bFromSweep :type Boolean) (SweepResult :type Hit%20Result%20Structure%20%28by%20ref%29))
  (if (Variables|Default|GetShowName)
    (Utilities|Casting|CastToP_CafeExplorer OtherActor)
    (bind _newtrack_0 (Timeline|Timeline_0 PlayFromStart)
      (:Update
        (bind _aswbp_interactable_name (Utilities|Casting|CastToWBP_InteractableName (UserInterface|GetUserWidgetObject (Variables|Default|GetWidget))))
        (Default|RenderOpacityIncrease _aswbp_interactable_name _newtrack_0)))))

(event OnComponentEndOverlap(Box)
  (params (OverlappedComponent :type Primitive%20Component%20Object%20Reference) (OtherActor :type Actor%20Object%20Reference) (OtherComp :type Primitive%20Component%20Object%20Reference) (OtherBodyIndex :type Integer))
  (if (Variables|Default|GetShowName)
    (Utilities|Casting|CastToP_CafeExplorer OtherActor)
    (bind _newtrack_0 (Timeline|Timeline_1 PlayFromStart)
      (:Update
        (bind _aswbp_interactable_name (Utilities|Casting|CastToWBP_InteractableName (UserInterface|GetUserWidgetObject (Variables|Default|GetWidget))))
        (Default|RenderOpacityDecrease _aswbp_interactable_name _newtrack_0)))))

(event Custom|HideWorldTextWidget
  (bind _newtrack_0 (Timeline|Timeline_1 PlayFromStart)
    (:Update
      (bind _aswbp_interactable_name (Utilities|Casting|CastToWBP_InteractableName (UserInterface|GetUserWidgetObject (Variables|Default|GetWidget))))
      (Default|RenderOpacityDecrease _aswbp_interactable_name _newtrack_0))))

(event EventBeginPlay
  (bind _aswbp_interactable_name (Utilities|Casting|CastToWBP_InteractableName (UserInterface|GetUserWidgetObject (Variables|Default|GetWidget))))
  (Variables|/Game/Blueprints/Widgets/WBP_InteractableName.WBP_InteractableName_C|SetName_Value _aswbp_interactable_name (Variables|Default|GetName)))

(event EventHighlight
  (params (OnOff :type Boolean))
  (Rendering|SetRenderCustomDepth (Variables|Default|GetMesh) OnOff))

(event EventInteract
  (CallFunction|InteractPrimary))

(event EventSecondaryAction
  (CallFunction|InteractSecondary))

(fn ConstructionScript)

(fn HighlightStaticMesh)

(fn InteractPrimary
  (Development|PrintString "interactable parent primary message"))

(fn InteractSecondary
  (Development|PrintString "interactable parent secondary message"))