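; BP_LightSwitch is an interactable switch that toggles lights across the whole level each time its Interact event fires.
; It flips LightOn, then applies it as visibility to every PointLight and SpotLight actor tagged "Toggable".
; It also sends TurnOnMessage or TurnOffMessage to all actors implementing I_Lights, finding every target by global actor search rather than stored references.
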(event EventBeginPlay)

(event Collision|EventActorBeginOverlap
  (params (OtherActor :type Actor%20Object%20Reference)))

(event EventTick
  (params (DeltaSeconds :type Float%20%28single-precision%29)))

(event EventInteract
  (Utilities|FlowControl|Sequence
    (:then_0
      (Variables|Default|SetLightOn (not (Variables|Default|GetLightOn))))
    (:then_1
      (bind _outactors (Actor|GetAllActorsOfClass "/Script/Engine.PointLight"))
      (for _array_element _outactors
        (if (Actor|ActorHasTag _array_element "Toggable")
          (Rendering|SetVisibility (Variables|/Script/Engine.Light|GetLightComponent _array_element) (Variables|Default|GetLightOn) false))))
    (:then_2
      (bind _outactors_2 (Actor|GetAllActorsOfClass "/Script/Engine.SpotLight"))
      (for _array_element_2 _outactors_2
        (if (Actor|ActorHasTag _array_element_2 "Toggable")
          (Rendering|SetVisibility (Variables|/Script/Engine.Light|GetLightComponent _array_element_2) (Variables|Default|GetLightOn) false))))
    (:then_3
      (bind _outactors_3 (Actor|GetAllActorswithInterface "/Game/Blueprints/Interfaces/I_Lights.I_Lights_C"))
      (if (Variables|Default|GetLightOn)
        (for _array_element_3 _outactors_3
          (Class|ILights|Turnon(Message) _array_element_3))
        (else
          (for _array_element_4 _outactors_3
            (Class|ILights|TurnOff(Message) _array_element_4)))))))

(fn ConstructionScript
  (|CallParentFunction))