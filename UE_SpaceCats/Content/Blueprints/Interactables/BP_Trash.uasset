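; BP_Trash is an interactable trash bin that disposes of whatever the cafe explorer player is carrying.
; On Interact it branches on the player's GameplayItemInHand enum state.
; One state simply switches to another, and a second clears the Ingredients list and destroys the actors in the held basket.
; Any other state destroys valid hand items and the cat item.
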(event EventBeginPlay
  (|CallParentFunction) ; This node is disabled and will not be called.\nDrag off pins to build functionality.
)

(event Collision|EventActorBeginOverlap
  (params (OtherActor :type Actor%20Object%20Reference)))

(event EventTick
  (params (DeltaSeconds :type Float%20%28single-precision%29)))

(event EventInteract
  (bind _asp_cafe_explorer (Utilities|Casting|CastToP_CafeExplorer (Game|GetPlayerCharacter 0)))
  (if (Utilities|Enum|Equal(Enum) (Variables|/Game/Blueprints/Player/P_CafeExplorer.P_CafeExplorer_C|GetGameplayItemInHand _asp_cafe_explorer) "NewEnumerator5")
    (Variables|/Game/Blueprints/Player/P_CafeExplorer.P_CafeExplorer_C|SetGameplayItemInHand _asp_cafe_explorer "NewEnumerator4")
    (elif (Utilities|Enum|Equal(Enum) (Variables|/Game/Blueprints/Player/P_CafeExplorer.P_CafeExplorer_C|GetGameplayItemInHand _asp_cafe_explorer) "NewEnumerator2")
      (Utilities|Array|Clear (Variables|/Game/Blueprints/Player/P_CafeExplorer.P_CafeExplorer_C|GetIngredients _asp_cafe_explorer))
      (for _array_element (Variables|/Game/Blueprints/Player/P_CafeExplorer.P_CafeExplorer_C|GetItemsInBasketHand _asp_cafe_explorer)
        (Utilities|IsValid _array_element
          (:Is%20Valid
            (Actor|DestroyActor _array_element))))
      (else
        (Utilities|IsValid (Variables|/Game/Blueprints/Player/P_CafeExplorer.P_CafeExplorer_C|GetIngredientHand1 _asp_cafe_explorer)
          (:Is%20Valid
            (Default|DestroyHandItems _asp_cafe_explorer))
          (:Is%20Not%20Valid
            _))
        (Default|DestroyCatItem _asp_cafe_explorer)))))

(fn ConstructionScript
  (|CallParentFunction))