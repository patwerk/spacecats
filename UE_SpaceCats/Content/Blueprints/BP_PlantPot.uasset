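; Interactable plant pot that grows through visual stages, from empty to a third and final plant stage.
; Interact advances the Stage enum one step, stopping at the last stage, and SecondaryAction resets it to empty.
; Both refresh through SwitchStageMesh, which shows only the static mesh matching the current stage.
; The construction script duplicates that visibility switch so the configured Stage shows in the editor.
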(event EventBeginPlay)

(event Collision|EventActorBeginOverlap
  (params (OtherActor :type Actor%20Object%20Reference)))

(event EventTick
  (params (DeltaSeconds :type Float%20%28single-precision%29)))

(event EventInteract
  (Utilities|IncreaseStage))

(event EventSecondaryAction
  (Utilities|Reset))

(fn ConstructionScript
  (switch Utilities|FlowControl|Switch|SwitchonE_IngredientStage (Variables|Default|GetStage)
    (:NewEnumerator0
      (Rendering|SetVisibility (Variables|Default|GetSM_Plant_Stage1) false false)
      (Rendering|SetVisibility (Variables|Default|GetSM_Plant_Stage2) false false)
      (Rendering|SetVisibility (Variables|Default|GetSM_Plant_Stage3) false false))
    (:NewEnumerator1
      (Rendering|SetVisibility (Variables|Default|GetSM_Plant_Stage1) true false)
      (Rendering|SetVisibility (Variables|Default|GetSM_Plant_Stage2) false false)
      (Rendering|SetVisibility (Variables|Default|GetSM_Plant_Stage3) false false))
    (:NewEnumerator2
      (Rendering|SetVisibility (Variables|Default|GetSM_Plant_Stage1) false false)
      (Rendering|SetVisibility (Variables|Default|GetSM_Plant_Stage2) true false)
      (Rendering|SetVisibility (Variables|Default|GetSM_Plant_Stage3) false false))
    (:NewEnumerator3
      (Rendering|SetVisibility (Variables|Default|GetSM_Plant_Stage1) false false)
      (Rendering|SetVisibility (Variables|Default|GetSM_Plant_Stage2) false false)
      (Rendering|SetVisibility (Variables|Default|GetSM_Plant_Stage3) true false))))