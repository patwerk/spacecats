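; BP_Ingredient_Pot is a plant pot with a selectable style and a sprout that grows in it.
; The construction script sets the pot mesh from PotStyle, choosing among three meshes.
; On BeginPlay, GrowthTimeline ticks a VInterpTo that eases the sprout's scale toward full size, using the timeline only as an update driver.
; A separate GrowPLant event makes the sprout visible, with no caller in this graph.
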(event Custom|GrowFirstSprout
  (Timeline|GrowthTimeline PlayFromStart
    (:Update
      (Transformation|SetRelativeScale3D (Variables|Default|GetSproutMesh) (Math|Interpolation|VInterpTo (Variables|/Script/Engine.SceneComponent|GetRelativeScale3D (Variables|Default|GetSproutMesh)) "1.000000,1.000000,1.000000" (Utilities|Time|GetWorldDeltaSeconds) 2.0)))))

(event Custom|GrowPLant
  (Rendering|SetVisibility (Variables|Default|GetSproutMesh) true false))

(event EventBeginPlay
  (CallFunction|GrowFirstSprout))

(fn ConstructionScript
  (switch Utilities|FlowControl|Switch|SwitchonE_PotStyle (Variables|Default|GetPotStyle)
    (:NewEnumerator0
      (Components|StaticMesh|SetStaticMesh (Variables|Default|GetPotStaticMesh) "/Game/meshes/static/plant_pots/pot_1.pot_1"))
    (:NewEnumerator1
      (Components|StaticMesh|SetStaticMesh (Variables|Default|GetPotStaticMesh) "/Game/meshes/static/plant_pots/pot_2.pot_2"))
    (:NewEnumerator2
      (Components|StaticMesh|SetStaticMesh (Variables|Default|GetPotStaticMesh) "/Game/meshes/static/plant_pots/pot_3.pot_3"))))